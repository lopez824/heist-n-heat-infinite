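; UI map manager actor that drives an indicator toward one object of a given class at a time.
; On BeginPlay it gathers all actors of ReferenceClass and spawns a UIController, passing it the indicator content and itself as player and initial item reference.
; Each tick it feeds the current object to the controller, advancing when that object becomes invalid.
; Once the list runs out, it destroys the controller and itself.
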(event `self.ReceiveBeginPlay`
  ;[1 1 1] Startup - Create Inidial UI Controller and Get All Item References
  (bind _outactors (`GameplayStatics.GetAllActorsOfClass` (`self.ReferenceClass`)))
  (set `self. ObjectReferences` _outactors)
  (bind _returnvalue (`|SpawnActorFromClass` "/Game/Blueprints/UIController.UIController_C" (`KismetMathLibrary.Conv_VectorToTransform` (`SceneComponent.K2_GetComponentLocation` (`self.DefaultSceneRoot`))) "Undefined" "OverrideRootScale" null null))
  (bind _output_get (set `self.UIController` _returnvalue))
  (set `/Game/Blueprints/UIController.ItemReference` self _output_get)
  (set `/Game/Blueprints/UIController.PlayerReference` self _output_get)
  (`/Game/Blueprints/UIController.UpdateIndicatorContent` _output_get (`self.IndicatorContent`)))

(event `self.ReceiveTick`
  (params (DeltaSeconds :type "Float (single-precision)"))
  (`self.UpdateItemReference`))

(event `UpdateItemReference`
  (bind _returnvalue (`KismetArrayLibrary.Array_Length` (`self. ObjectReferences`)))
  (bind _output (`|GetArrayItem` (`self. ObjectReferences`) (`self.IndicateIndex`)))
  ;[1 1 1] Just Call This every tick, ugly but useful
  (if (`KismetSystemLibrary.IsValid` _output)
    (set `/Game/Blueprints/UIController.ItemReference` _output (`self.UIController`) :!label _label)
    (else
      (bind _output_get (set `self.IndicateIndex` (`KismetMathLibrary.Min` (+ (`self.IndicateIndex`) 1) _returnvalue)))
      (if (< _output_get _returnvalue)
        (goto _label)
        (else
          (`self.K2_DestroyActor` (`self.UIController`))
          (`self.K2_DestroyActor`))))))

(fn `UserConstructionScript`)