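; Player vehicle for a driving game where fuel doubles as health: it drains over time, is spent on boosts and is lost to cop crashes and missiles.
; Input drives throttle, drift steering and boost, while Tick applies speed limits, roll clamping, speed-based audio and FOV, and a state machine that eases the camera between tagged viewpoints.
; Fuel tanks refill fuel, five safe boxes trigger an ending, and empty fuel explodes the car before the death menu.
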(event `AngleStabilizer`
  (bind _anglex_limit (`self.AngleX_Limit`))
  (bind _returnvalue (- 0.0 _anglex_limit))
  (bind _roll (.roll (.rotation (`self.GetTransform`))))
  (bind _returnvalue_2 (> _roll _anglex_limit))
  ;[1 1 1] Limit the X rotation to a range
  (if (or _returnvalue_2 (< _roll _returnvalue))
    (`self.K2_SetActorTransform` (`KismetMathLibrary.MakeTransform` (.location (`self.GetTransform`)) (`KismetMathLibrary.MakeRotator` (`KismetMathLibrary.SelectFloat` _anglex_limit _returnvalue _returnvalue_2) (.pitch (.rotation (`self.GetTransform`))) (.yaw (.rotation (`self.GetTransform`)))) (.scale (`self.GetTransform`))))))

(event `UpdateBaseVelocity`
  (bind (_returnvalue_x _returnvalue_y) (`KismetMathLibrary.BreakVector` (`self.GetVelocity`)))
  (bind _boostbasevelocity_x (`KismetMathLibrary.BreakVector` (`self.BoostBaseVelocity`)))
  ;[1 1 1] Base Boost
  (if (not (or (> (`KismetMathLibrary.Abs` _returnvalue_x) _boostbasevelocity_x) (> (`KismetMathLibrary.Abs` _returnvalue_y) _boostbasevelocity_x)))
    (`ArcadeVehicleMovementComponentBase.SetVehicleLinearVelocity` (`self.MovementComponent`) (`self.BoostBaseVelocity`) false)))

(event `UpdateDriftingAudio`
  ;[1 1 1] Audio - Engine
  (`AudioComponent.SetFloatParameter` (`self.Drifting`) "RPM" (`KismetMathLibrary.MapRangeClamped` (`ArcadeVehicleMovementComponentBase.GetCurrentSpeed` (`self.MovementComponent`)) 0.0 100.0 0.0 1.0)))

(event `UpdateEngineForwardAudio`
  ;[1 1 1] Audio - Engine
  (`AudioComponent.SetFloatParameter` (`self.EngineAudio_Forward`) "RPM" (`self.ForwardForce`)))

(event `StartBoostAudio`
  (bind _boost (`self.Boost`))
  ;[1 1 1] Boost Audio
  (`AudioComponent.Play` _boost 0.0)
  (`AudioComponent.AdjustVolume` _boost 1.0 1.0 "Linear"))

(event `SpawnTrail`
  ;[1 1 1] Car Control
  (`self.Spawn Wheel Trail` (`self.Wheel_Rear_Right`))
  (`self.Spawn Wheel Trail` (`self.Wheel_Rear_Left`)))

(event `UpdateEngineAudio`
  ;[1 1 1] Audio - Engine
  (bind _output_get (set `self.RPM` (`CurveFloat.GetFloatValue` (`self.EngineMainAudioCurve`) (`KismetMathLibrary.MapRangeClamped` (`ArcadeVehicleMovementComponentBase.GetCurrentSpeed` (`self.MovementComponent`)) 0.0 100.0 0.0 1.0))))
  (`AudioComponent.SetFloatParameter` (`self.EngineAudio`) "RPM" _output_get))

(event `InputAction|Boost`
  (params (Key :type "Key Structure"))
  (bind _returnvalue (- (`self.Fuel_Current`) 20))
  ;[1 1 1] Boost Visual
  (:`Pressed`
    (if (> _returnvalue 0)
      (`self.StartBoostAudio`)
      (`self.UpdateBaseVelocity`)
      (set `self.Fuel_Current` _returnvalue)
      (bind _asplay_hud (cast `/Game/Blueprints/PlayHUD` (`PlayerController.GetHUD` (`GameplayStatics.GetPlayerController` 0))))
      (`/Game/Blueprints/PlayHUD.Update_UI` _asplay_hud)
      (set `self.IsBoosting` true)
      (`SceneComponent.SetVisibility` (`self.Exhaust`) true false)
      (`SceneComponent.SetVisibility` (`self.Wind`) true false)
      (bind (_direction _acceleration) (`Timeline|IncreaseBoost` :!via `PlayFromStart`)
        (:`Update`
          (`SceneComponent.SetWorldScale3D` (`self.Exhaust`) _acceleration)
          (`SceneComponent.SetWorldScale3D` (`self.Wind`) _acceleration)))
      (else
        (set `self.IsBoosting` false))))
  (:`Released`
    (`self.EndBoostAudio`)
    (set `self.IsBoosting` false)
    (bind (_direction_2 _acceleration_2) (`Timeline|DecreaseBoost` :!via `PlayFromStart`)
      (:`Update`
        (`SceneComponent.SetWorldScale3D` (`self.Exhaust`) _acceleration_2)
        (`SceneComponent.SetWorldScale3D` (`self.Wind`) _acceleration_2))
      (:`Finished`
        (`SceneComponent.SetVisibility` (`self.Exhaust`) false false)
        (`SceneComponent.SetVisibility` (`self.Wind`) false false)))))

(event `InputAxis|Throttle`
  (params (AxisValue :type "Float (single-precision)"))
  (bind _movementcomponent (`self.MovementComponent`))
  ;[1 1 1] Car Control
  (if (`self.IsGameStart`)
    (`|ExecutionSequence`
      (:`then_0`
        ;;[1 1 1] Set Engine Forward Parameter
        (if (>= (`KismetMathLibrary.Abs` AxisValue) 0.7)
          (bind (_direction _alpha) (`Timeline|ForwardForceAlpha` :!label _label)
            (:`Update`
              (set `self.ForwardForce` _alpha)))
          (else
            (goto _label :!via `Reverse`))))
      (:`then_1`
        (if (== (`KismetMathLibrary.Abs` (stale `InputAxis|Steering` AxisValue)) 1.0)
          (`ArcadeVehicleMovementComponentBase.SetAccelerationInput` _movementcomponent (/ AxisValue 5.0))
          (else
            (`ArcadeVehicleMovementComponentBase.SetAccelerationInput` _movementcomponent AxisValue)))))))

(event `EndBoostAudio`
  ;[1 1 1] Boost Audio
  (`AudioComponent.AdjustVolume` (`self.Boost`) 1.0 0.0 "Linear"))

(event `PlayDriftingAudio`
  ;[1 1 1] Car Control
  (`AudioComponent.AdjustVolume` (`self.Drifting`) 0.1 1.0 "Linear"))

(event `Update Boost`
  (bind _returnvalue (`self.GetVelocity`))
  (bind _returnvalue_2 (`self.GetVelocity`))
  (bind _maxspeed (`self.MaxSpeed`))
  (bind _maxboostspeed (`self.MaxBoostSpeed`))
  ;[1 1 1] Boost Implementation
  (if (`self.IsBoosting`)
    (if (> (`KismetMathLibrary.VSize` _returnvalue) _maxboostspeed)
      (`PrimitiveComponent.SetPhysicsLinearVelocity` (`self.VehicleMesh`) (* (`KismetMathLibrary.Normal` _returnvalue) _maxboostspeed) false "None")
      (else
        (`PrimitiveComponent.SetPhysicsLinearVelocity` (`self.VehicleMesh`) (* (`self.GetVelocity`) (`self.BoostModifier`)) false "None")))
    (elif (> (`KismetMathLibrary.VSize` _returnvalue_2) _maxspeed)
      (`PrimitiveComponent.SetPhysicsLinearVelocity` (`self.VehicleMesh`) (* (`KismetMathLibrary.Normal` _returnvalue_2) _maxspeed) false "None"))))

(event `InputAxis|Steering`
  (params (AxisValue :type "Float (single-precision)"))
  (bind _movementcomponent (`self.MovementComponent`))
  ;[1 1 1] Car Control
  (if (`self.IsGameStart`)
    (`|ExecutionSequence`
      (:`then_0`
        (`ArcadeVehicleMovementComponentBase.SetTurningInput` (`self.MovementComponent`) AxisValue)
        (if (== (`KismetMathLibrary.Abs` AxisValue) 1.0)
          (`ArcadeVehicleMovementComponentBase.SetDriftInput` _movementcomponent true)
          (`self.PlayDriftingAudio`)
          (`self.SpawnTrail`)
          (else
            (`ArcadeVehicleMovementComponentBase.SetDriftInput` _movementcomponent false)
            (`self.StopDriftingAudio`))))
      (:`then_1`
        ;;[1 1 1] Set Engine Forward Parameter
        (if (>= (`KismetMathLibrary.Abs` AxisValue) 0.7)
          (bind (_direction _alpha) (`Timeline|SteerForceAlpha` :!label _label_2)
            (:`Update`
              (set `self.SteerForce` _alpha)))
          (else
            (goto _label_2 :!via `Reverse`)))))))

(event `StopDriftingAudio`
  ;[1 1 1] Car Control
  (`AudioComponent.AdjustVolume` (`self.Drifting`) 0.3 0.001 "Linear"))

(event `InputAction|SwitchCamera`
  (params (Key :type "Key Structure"))
  ;[1 1 1] Test
  (:`Pressed`
    (`self.ViewpointCycle`)))

(event `self.ReceiveTick`
  (params (DeltaSeconds :type "Float (single-precision)"))
  ;[1 1 1] State Machine - Every Frame
  (`self.UpdateFireVFX`)
  (`|ExecutionSequence`
    (:`then_0`
      (if (`self.IsGameStart`)
        (if (`self.IsGameOver`)
          ;;[1 1 1] Game End
          (bind _output_get (set `self.CallFunctionTimer` (+ DeltaSeconds (`self.CallFunctionTimer`))))
          (if (> _output_get 2.0)
            (`self.CallGameEnd`))
          (else
            (`self.DetectGameEnd`)
            (`self.ResetCollide` DeltaSeconds)
            (set `self.CallFunctionTimer` 0.0)
            (`|ExecutionSequence`
              (:`then_0`
                (`self.Update Boost`))
              (:`then_1`
                (`self.Update State Machine`))
              (:`then_2`
                (`self.Update Camera Rotation`))
              (:`then_3`
                (`self.Update FOV`)))))
        (else
          ;;[1 1 1] Loop Run
          (`ArcadeVehicleMovementComponentBase.SetAccelerationInput` (`self.MovementComponent`) 1.0)
          (set `self.ForwardForce` 0.5)
          (`SceneComponent.K2_SetWorldRotation` :`self` (`self.VehicleMesh`)))))
    (:`then_1`
      (`self.Update Audio`))
    (:`then_2`
      (`self.AngleStabilizer`))))

(event `Key|H`
  (params (Key :type "Key Structure"))
  ;[1 1 1] Test
  (:`Pressed`
    (set `self.IsGameStart` true)))

(event `Update State Machine`
  ;[1 1 1] State Machine - Every Frame
  ;;[1 1 1] Camera State Machine Checked Every Tick
  (switch `name` (`self.ViewpointState`)
    (:`START`
      (`SceneComponent.K2_DetachFromComponent` (`self.Camera`) "KeepWorld" "KeepWorld" "KeepWorld" true)
      (set `self.ViewpointState` "UPDATE"))
    (:`UPDATE`
      (`self.ViewpointInterpolate`))
    (:`STOP`
      (`self.ViewpointUnsnap`))))

(event `Update Camera Rotation`
  (bind (_returnvalue_roll _returnvalue_pitch _returnvalue_yaw) (`KismetMathLibrary.BreakRotator` (`SceneComponent.K2_GetComponentRotation` (`self.VehicleMesh`))))
  (bind _output (`|GetArrayItem` (`self.Viewpoints`)))
  (bind (_returnvalue_roll_2 _returnvalue_pitch_2) (`KismetMathLibrary.BreakRotator` (`SceneComponent.K2_GetComponentRotation` _output)))
  ;[1 1 1] State Machine - Every Frame
  ;;[1 1 1] Set The viewpoint rorate with player when using the TPS Vehicle Perspective
  (`SceneComponent.K2_SetWorldRotation` _output (`KismetMathLibrary.MakeRotator` _returnvalue_roll_2 _returnvalue_pitch_2 _returnvalue_yaw) false false))

(event `self.ReceiveBeginPlay`
  ;[1 1 1] State Machine - Initial all viewpoints and set first camera to default viewpoint
  (`self.ResetSafes`)
  (`self.SetExplosionVFXVisibility`)
  (`|ExecutionSequence`
    (:`then_0`
      (bind _output_get (set `self.Viewpoints` (`self.GetComponentsByTag` "/Script/Engine.ArrowComponent" "viewpoint")))
      (`SceneComponent.K2_AttachToComponent` (`self.Camera`) (`|GetArrayItem` _output_get (`self.ViewpointIndex`)) "None" "SnapToTarget" "SnapToTarget" "SnapToTarget" true))
    (:`then_1`
      (set `self.ViewpointPositions` (`self.GetComponentsByTag` "/Script/Engine.SpringArmComponent" "position")))
    (:`then_2`
      (`KismetSystemLibrary.Delay` 2.0 :!label _label_3)
      (if (`self.IsGameStart`)
        (set `self.Fuel_Current` (- (`self.Fuel_Current`) 1))
        (bind _asplay_hud (cast `/Game/Blueprints/PlayHUD` (`PlayerController.GetHUD` (`GameplayStatics.GetPlayerController` 0))))
        (`/Game/Blueprints/PlayHUD.Update_UI` _asplay_hud)
        (goto _label_3)
        (else
          (goto _label_3))))
    (:`then_3`
      (`self.StopDriftingAudio`))))

(event `Update FOV`
  ;[1 1 1] State Machine - Every Frame
  ;;[1 1 1] FOV Settings
  (if (`self.IsGameStart`)
    (`CameraComponent.SetFieldOfView` (`self.Camera`) (`KismetMathLibrary.MapRangeClamped` (`ArcadeVehicleMovementComponentBase.GetCurrentSpeed` (`self.MovementComponent`)) 60.0 100.0 100.0 110.0))))

(event `Update Audio`
  ;[1 1 1] State Machine - Every Frame
  ;;[1 1 1] Update Audio
  (`self.UpdateEngineAudio`)
  (`self.UpdateEngineForwardAudio`)
  (`self.UpdateDriftingAudio`))

(event `ViewpointInterpolate`
  (bind _returnvalue (`SceneComponent.K2_GetComponentToWorld` (`|GetArrayItem` (`self.Viewpoints`) (`self.ViewpointIndex`))))
  (bind _result (`|EaseFunction` "SinusoidalIn" (`self.CemeraLerp`) (`SceneComponent.GetRelativeTransform` (`self.Camera`)) _returnvalue))
  ;[1 1 1] State Machine - Ease Camera Position Based On index, and cease to swtich state
  (`SceneComponent.K2_SetRelativeTransform` (`self.Camera`) _result false false)
  (if (< (`KismetMathLibrary.Vector_Distance` (.location _result) (.location _returnvalue)) 1.0)
    (set `self.ViewpointState` "STOP")
    (else
      (set `self.ViewpointState` "UPDATE"))))

(event `ViewpointUnsnap`
  ;[1 1 1] State Machine - Other States
  (`SceneComponent.K2_DetachFromComponent` (`self.Camera`) "KeepWorld" "KeepWorld" "KeepWorld" true)
  (set `self.ViewpointState` "UPDATE"))

(event `ViewpointCycle`
  ;[1 1 1] State Machine - Other States
  (set `self.ViewpointIndex` (mod (+ (`self.ViewpointIndex`) 1) (`KismetArrayLibrary.Array_Length` (`self.Viewpoints`))))
  (set `self.ViewpointState` "START"))

(event `CollectFuelTank`
  (bind _returnvalue (+ (`self.Fuel_Current`) (`self.FuelTankVolume`)))
  ;[1 1 1] Interaction
  (set `self.Fuel_Current` (`KismetMathLibrary.SelectInt` (`self.Fuel_Max`) _returnvalue (> _returnvalue (`self.Fuel_Max`))))
  (bind _result (`/Engine/EditorBlueprintResources/StandardMacros.IncrementInt` (`self.Cnt_FuelTank`))
    (:`  `
      (`KismetSystemLibrary.PrintString` (`KismetStringLibrary.BuildString_Int` "Fuel Tank Collected: " "" _result))
      (bind _asplay_hud (cast `/Game/Blueprints/PlayHUD` (`PlayerController.GetHUD` (`GameplayStatics.GetPlayerController` 0))))
      (`/Game/Blueprints/PlayHUD.Update_UI` _asplay_hud)
      (`AudioComponent.Play` (`self.CollectSound`) 0.0))))

(event `ViewpointHome`
  ;[1 1 1] State Machine - Other States
  (set `self.ViewpointIndex` 0)
  (set `self.ViewpointState` "START"))

(event `CollectSafeBox`
  ;[1 1 1] Interaction
  (bind _result (`/Engine/EditorBlueprintResources/StandardMacros.IncrementInt` (`self.Cnt_SafeBox`))
    (:`  `
      (`|ExecutionSequence`
        (:`then_0`
          (`KismetSystemLibrary.PrintString` (`KismetStringLibrary.BuildString_Int` "Safe Box Collected: " "" _result))
          (bind _asplay_hud (cast `/Game/Blueprints/PlayHUD` (`PlayerController.GetHUD` (`GameplayStatics.GetPlayerController` 0))))
          (`/Game/Blueprints/PlayHUD.Update_UI` _asplay_hud)
          (`SceneComponent.SetVisibility` (`|GetArrayItem` (`self.SafesModelArray`) (`self.CurrentSafeIndex`)) true false)
          (set `self.CurrentSafeIndex` (+ (`self.CurrentSafeIndex`) 1))
          (if (> (`self.CurrentSafeIndex`) 0)
            (`SceneComponent.SetVisibility` (`self.Dollar`) true false)
            (`ActorComponent.SetActive` (`self.Dollar`) true false)
            (`AudioComponent.Play` (`self.CollectSound`) 0.0)))
        (:`then_1`
          (`self.CheckSafeCount`))))))

(event `CheckSafeCount`
  ;[1 1 1] Ending UI Message
  (if (== (`self.Cnt_SafeBox`) 5)
    (bind _returnvalue (`|CreateWidget` "/Game/Blueprints/BP_UI_Ending.BP_UI_Ending_C" (`GameplayStatics.GetPlayerController` 0)))
    (bind _output_get (set `self.uiEndingReference` _returnvalue))
    (`UserWidget.AddToViewport` _output_get 0)
    (`|ExecutionSequence`
      (:`then_0`
        (`KismetSystemLibrary.Delay` 3.0)
        (`Widget.RemoveFromParent` (`self.uiEndingReference`)))
      (:`then_1`
        (bind _returnvalue_2 (`GameplayStatics.GetActorOfClass` "/Game/AudioResources/BP_Music.BP_Music_C"))
        (`/Game/AudioResources/BP_Music.FinalStage` _returnvalue_2)))))

(event `Key|Escape`
  (params (Key :type "Key Structure"))
  ;[1 1 1] Pause Menu
  (:`Pressed`
    (bind _asplay_hud (cast `/Game/Blueprints/PlayHUD` (`PlayerController.GetHUD` (`GameplayStatics.GetPlayerController` 0)) :!label _label_4))
    (`/Game/Blueprints/PlayHUD.Call Paused Menu` _asplay_hud true "You Paused")))

(event `Key|P`
  (params (Key :type "Key Structure"))
  ;[1 1 1] Pause Menu
  (:`Pressed`
    (goto _label_4)))

(event `self.CrashCollide.OnComponentHit`
  (params (HitComponent :type "PrimitiveComponent Object Reference") (OtherActor :type "Actor Object Reference") (OtherComp :type "PrimitiveComponent Object Reference") (NormalImpulse :type "Vector Structure") (Hit :type "HitResult Structure (by ref)"))
  ;[1 1 1] Collide System
  (bind _asnew_cop (cast `/Game/Blueprints/NewCop` OtherActor))
  ;;[1 1 1] Debug Log
  (`KismetSystemLibrary.PrintString` (`KismetStringLibrary.Conv_DoubleToString` (`ArcadeVehicleMovementComponentBase.GetLastAppliedAcceleration` (`StaticArcadeVehiclePawn.MovementComponent` _asnew_cop))))
  (if (not (`self.IsCollide`))
    (bind _outhit (`KismetSystemLibrary.LineTraceSingle` :`Start` (`SceneComponent.K2_GetComponentLocation` (`StaticArcadeVehiclePawn.VehicleMesh` _asnew_cop)) :`End` (`SceneComponent.K2_GetComponentLocation` (`self.VehicleMesh`)) :`TraceChannel` "TraceTypeQuery1" :`DrawDebugType` "Persistent" :`bIgnoreSelf` false))
    (`NiagaraFunctionLibrary.SpawnSystemAtLocation` (`self.CollideVFX`) (`.Location` (`GameplayStatics.BreakHitResult` _outhit)))
    (`KismetSystemLibrary.PrintString` "Crash!")
    (`AudioComponent.Play` (`self.Collision`) 0.0)
    (bind _output_get (set `self.Fuel_Current` (- (`self.Fuel_Current`) 20)))
    (set `self.IsCollide` true)
    (if (< _output_get 0)
      (set `self.Fuel_Current` 0))
    (bind _asplay_hud (cast `/Game/Blueprints/PlayHUD` (`PlayerController.GetHUD` (`GameplayStatics.GetPlayerController` 0))))
    (`/Game/Blueprints/PlayHUD.Update_UI` _asplay_hud)))

(event `self.CrashCollide.OnComponentBeginOverlap`
  (params (OverlappedComponent :type "PrimitiveComponent Object Reference") (OtherActor :type "Actor Object Reference") (OtherComp :type "PrimitiveComponent Object Reference") (OtherBodyIndex :type Integer) (bFromSweep :type Boolean) (SweepResult :type "HitResult Structure (by ref)"))
  ;[1 1 1] Collide System
  (cast `/Game/Blueprints/BP_Missle` OtherActor)
  (`KismetSystemLibrary.PrintString` "Hit a missile" true true (struct :`R` 0.973958 :`G` 0.030436 :`B` 0.131531 :`A` 1.0))
  (bind _output_get (set `self.Fuel_Current` (- (`self.Fuel_Current`) 20)))
  (if (< _output_get 0)
    (set `self.Fuel_Current` 0))
  (bind _asplay_hud (cast `/Game/Blueprints/PlayHUD` (`PlayerController.GetHUD` (`GameplayStatics.GetPlayerController` 0))))
  (`/Game/Blueprints/PlayHUD.Update_UI` _asplay_hud))

(fn `CallGameEnd`
  (bind _asplay_hud (cast `/Game/Blueprints/PlayHUD` (`PlayerController.GetHUD` (`GameplayStatics.GetPlayerController` 0))))
  (`/Game/Blueprints/PlayHUD.Call Paused Menu` _asplay_hud false "You Died"))

(fn `DetectGameEnd`
  (if (not (> (`self.Fuel_Current`) 0))
    (`KismetSystemLibrary.PrintString` "GameOver")
    (`self.SetExplosionVFXVisibility`)
    (`ActorComponent.Activate` (`self.ExplosionVFX`) true)
    (set `self.IsGameOver` true)
    (`SceneComponent.SetVisibility` (`self.Dollar`) false false)
    (for _array_element (`|MakeArray` (`self.Wheel_Front_Left`) (`self.Wheel_Rear_Right`) (`self.Wheel_Front_Right`) (`self.Wheel_Rear_Left`) (`self.Safe1`) (`self.Safe2`) (`self.Safe3`) (`self.Safe4`) (`self.Safe5`))
      (`SceneComponent.SetVisibility` _array_element false false)
      (`AudioComponent.Play` (`self.Explosion`) 0.0))
    (`StaticMeshComponent.SetStaticMesh` (`self.VehicleVisualMesh`) "/Game/Vehicles/SportsCar/Mesh/TestRed_2.TestRed_2")
    (`PrimitiveComponent.SetMaterial` (`self.VehicleVisualMesh`) 0 "/Game/Vehicles/Materials/NM_Burnt.NM_Burnt")))

(fn `ResetCollide`
  (params (B :type "Float (double-precision)"))
  (if (`self.IsCollide`)
    (bind _output_get (set `self.CollideTimer` (+ (`self.CollideTimer`) B)))
    (if (>= _output_get 5.0)
      (set `self.IsCollide` false)
      (set `self.CollideTimer` 0.0))))

(fn `ResetSafes`
  (set `self.CurrentSafeIndex` 0)
  (bind _output_get (set `self.SafesModelArray` (`|MakeArray` (`self.Safe1`) (`self.Safe2`) (`self.Safe3`) (`self.Safe4`) (`self.Safe5`))))
  (for _array_element _output_get
    (`SceneComponent.SetVisibility` _array_element false false))
  (`SceneComponent.SetVisibility` (`self.Dollar`) false false)
  (`ActorComponent.SetActive` (`self.Dollar`) false false)
  (`SceneComponent.SetVisibility` (`self.Fire`) false false))

(fn `SetExplosionVFXVisibility`
  (if (> (`self.Fuel_Current`) 0)
    (`SceneComponent.SetVisibility` (`self.ExplosionVFX`) false false)
    (else
      (`SceneComponent.SetVisibility` (`self.ExplosionVFX`) true false))))

(fn `Spawn Wheel Trail`
  (params (`Wheel Reference` :type "SceneComponent Object Reference"))
  (bind _returnvalue (`SceneComponent.K2_GetComponentLocation` `Wheel Reference`))
  (if (`KismetMathLibrary.InRange_FloatFloat` (.z _returnvalue) -50.0 40.0)
    (`GameplayStatics.SpawnEmitterAtLocation` "/Game/Vehicles/Materials/TireTrail.TireTrail" _returnvalue)))

(fn `UpdateFireVFX`
  (if (< (`self.Fuel_Current`) 30)
    (`SceneComponent.SetVisibility` (`self.Fire`) true false)
    (else
      (`SceneComponent.SetVisibility` (`self.Fire`) false false))))

(fn `UserConstructionScript`
  (`parent.UserConstructionScript`))