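; BP_Missle is a missile actor that plays start and end cues, likely audio, around its impact.
; BeginPlay triggers the Start component.
; The Rocket component's first hit, gated by DoOnce, hides the rocket, spawns an NS_Poof Niagara effect below its location and triggers the End component.
; It also unhides the root without propagating to children, then destroys the actor after a short delay.
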(event `self.rocket.OnComponentHit`
  (params (HitComponent :type "PrimitiveComponent Object Reference") (OtherActor :type "Actor Object Reference") (OtherComp :type "PrimitiveComponent Object Reference") (NormalImpulse :type "Vector Structure") (Hit :type "HitResult Structure (by ref)"))
  (bind _rocket (`self.rocket`))
  (`/Engine/EditorBlueprintResources/StandardMacros.DoOnce` false
    (:`Completed`
      (`SceneComponent.SetVisibility` _rocket false false)
      (`NiagaraFunctionLibrary.SpawnSystemAtLocation` "/Game/Niagara/VFX/NS_Poof.NS_Poof" (+ (`SceneComponent.K2_GetComponentLocation` _rocket) (0.0 0.0 -200.0)))
      (`self.PlayBombEnd`)
      (`SceneComponent.SetHiddenInGame` (`self.DefaultSceneRoot`) false false)
      (`KismetSystemLibrary.Delay` 4.0)
      (`self.K2_DestroyActor`))))

(event `PlayBombEnd`
  (`AudioComponent.Play` (`self.End`) 0.0))

(event `PlayBombStart`
  (`AudioComponent.Play` (`self.Start`) 0.0))

(event `self.ReceiveBeginPlay`
  (`self.PlayBombStart`))

(fn `UserConstructionScript`)