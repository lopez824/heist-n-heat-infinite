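; NewCop is an AI police car that patrols set points and can switch to pursuit.
; It writes patrol point locations to its AI Blackboard and drives a movement component through acceleration and turning inputs, drifting at full lock.
; While pursuing, Tick snaps its yaw toward the first NewCar found, standing in for a Behavior Tree RotateTo task and searching all actors of that class every frame.
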(event `self.ReceiveTick`
  (params (DeltaSeconds :type "Float (single-precision)"))
  ;[1 1 1] Replaces RotateTo task in Behavior Tree
  (if (`self.InPursuit`)
    (bind _outactors (`GameplayStatics.GetAllActorsOfClass` "/Game/Blueprints/NewCar.NewCar_C"))
    (`self.UpdateRotation` (`|GetArrayItem` _outactors))))

(event `self.ReceiveBeginPlay`
  ;[1 1 1] Start Patrolling
  (`self.SetPatrolLocation` 0))

(fn `GetPatrolLocation`
  (returns (PatrolLocation :type "Vector Structure"))
  ;[1 1 1] Gets AI Blackboard PatrolLocation value
  (return (`BlackboardComponent.GetValueAsVector` (`AIController.Blackboard` (`AIBlueprintHelperLibrary.GetAIController` self)) (`self.PatrolLocation`))))

(fn `IsPursuing`
  (params (isPursuing :type Boolean))
  (set `self.InPursuit` isPursuing))

(fn `SetPatrolLocation`
  (params (PatrolIndex :type Integer))
  (bind _output (`|GetArrayItem` (`self.PatrolPoints`) PatrolIndex))
  ;[1 1 1] Sets AI Blackboard PatrolLocation value
  (if (`KismetSystemLibrary.IsValid` _output)
    (`BlackboardComponent.SetValueAsVector` (`AIController.Blackboard` (`AIBlueprintHelperLibrary.GetAIController` self)) (`self.PatrolLocation`) (`self.K2_GetActorLocation` _output))
    (`self.UpdateAcceleration` 0.25)))

(fn `UpdateAcceleration`
  (params (NewAcceleration :type "Float (double-precision)"))
  (`ArcadeVehicleMovementComponentBase.SetAccelerationInput` (`self.MovementComponent`) NewAcceleration))

(fn `UpdateRotation`
  (params (LookAtActor :type "Actor Object Reference"))
  (bind (_returnvalue_roll _returnvalue_pitch) (`KismetMathLibrary.BreakRotator` (`self.K2_GetActorRotation`)))
  (bind (_returnvalue_roll_2 _returnvalue_pitch_2 _returnvalue_yaw) (`KismetMathLibrary.BreakRotator` (`KismetMathLibrary.FindLookAtRotation` (`self.K2_GetActorLocation`) (`self.K2_GetActorLocation` LookAtActor))))
  (`self.K2_SetActorRotation` (`KismetMathLibrary.MakeRotator` _returnvalue_roll _returnvalue_pitch _returnvalue_yaw)))

(fn `UpdateTurning`
  (params (NewTurn :type "Float (double-precision)"))
  (bind _movementcomponent (`self.MovementComponent`))
  (`ArcadeVehicleMovementComponentBase.SetTurningInput` (`self.MovementComponent`) NewTurn)
  (if (== (`KismetMathLibrary.Abs` NewTurn) 1.0)
    (`ArcadeVehicleMovementComponentBase.SetDriftInput` _movementcomponent true)
    (else
      (`ArcadeVehicleMovementComponentBase.SetDriftInput` _movementcomponent false))))

(fn `UserConstructionScript`
  (`self.UpdateAcceleration` 0.25))