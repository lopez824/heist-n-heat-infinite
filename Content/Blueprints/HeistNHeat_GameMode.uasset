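; Game mode for Heist N Heat that lets Twitch chat spawn obstacles, ramps, fuel tanks or missile rain around the player's car.
; Twitch_Influence matches message keywords and, subject to a minimum interval, credits the sender on the HUD and spawns the item.
; Obstacles and missiles use random half-circle sectors, retrying blocked spawns, with missile distance scaling with car speed.
; Ramps and fuel spawn at the car's SpawnPoint; timed cleanup is unconnected.
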(event `self.ReceiveBeginPlay`
  (bind _returnvalue (`GameplayStatics.GetActorOfClass` "/Script/TwitchIntegrator.twitchChat"))
  (set `self.Actor_TwitchIntegration` _returnvalue))

(event `Twitch_Influence`
  (params (UserID :type String) (TwitchMessage :type String))
  (bind _returnvalue (`KismetSystemLibrary.GetGameTimeInSeconds`))
  (bind _twitchmessage (`self.TwitchMessage`))
  ;[1 1 1] Generate Item by Twitch
  (set `self.UserID` UserID)
  (set `self.TwitchMessage` TwitchMessage)
  (`|ExecutionSequence`
    (:`then_0`
      (set `self.TwitchCommand` -1))
    (:`then_1`
      (if (`KismetStringLibrary.Contains` _twitchmessage "block")
        (set `self.TwitchCommand` 0)))
    (:`then_2`
      (if (`KismetStringLibrary.Contains` _twitchmessage "ramp")
        (set `self.TwitchCommand` 1)))
    (:`then_3`
      (if (`KismetStringLibrary.Contains` _twitchmessage "fuel")
        (set `self.TwitchCommand` 2)))
    (:`then_4`
      (if (`KismetStringLibrary.Contains` _twitchmessage "missile")
        (set `self.TwitchCommand` 3)))
    (:`then_5`
      (switch `int` (`self.TwitchCommand`)
        (:`0`
          (set `self.ItemDescription` "some obstacles"))
        (:`1`
          (set `self.ItemDescription` "a ramp"))
        (:`2`
          (set `self.ItemDescription` "a fuel tank"))
        (:`3`
          (set `self.ItemDescription` "a missile rain")))
      (bind _asplay_hud (cast `/Game/Blueprints/PlayHUD` (`PlayerController.GetHUD` (`GameplayStatics.GetPlayerController` 0))))
      (if (>= (- _returnvalue (`self.Time_LastAdd`)) (`self.Time_MinInterval`))
        (set `self.Time_LastAdd` _returnvalue)
        (`/Game/Blueprints/PlayHUD.Update_UI_Twitch` _asplay_hud (`self.UserID`) (`KismetStringLibrary.Concat_StrStr` "sent " (`self.ItemDescription`) "!"))
        (switch `int` (`self.TwitchCommand`)
          (:`0`
            (`self.Add The Obstacle`))
          (:`1`
            (`self.Add The Ramp`))
          (:`2`
            (`self.Add The Fuel`))
          (:`3`
            (`self.Add The Missile`)))))))

(event `Add The Obstacle`
  ;[1 1 1] Generate Item by Twitch
  (`KismetSystemLibrary.PrintString` "Add an obstacle")
  (set `self.Item_AskedByTwitch` (`self.Class_Obstacle`))
  (for _ (range 1 6)
    (`self.SpawnObstacle`)
    (`AudioComponent.Play` (`self.TwitchHint`) 0.0 :!label _label)))

(event `Add The Ramp`
  ;[1 1 1] Generate Item by Twitch
  (`KismetSystemLibrary.PrintString` "Add a ramp")
  (set `self.Item_AskedByTwitch` (`self.Class_Ramp`))
  (`self.SpawnRamp`)
  (goto _label))

(event `Add The Fuel`
  ;[1 1 1] Generate Item by Twitch
  (`KismetSystemLibrary.PrintString` "Add a fuel tank")
  (set `self.Item_AskedByTwitch` (`self.Class_Fuel`))
  (`self.SpawnFuel`)
  (goto _label))

(event `Add The Missile`
  ;[1 1 1] Generate Item by Twitch
  (`KismetSystemLibrary.PrintString` "Add an missile rain")
  (set `self.Item_AskedByTwitch` (`self.Class_Missile`))
  (for _ (range 1 6)
    (`self.SpawnMissile`)
    (goto _label)))

(event `SpawnObstacle`
  ;[1 1 1] Generate Item by Twitch
  (set `self.Cnt_Spawn` 0)
  (set `self.AngleRange` (/ 180.0 (`KismetMathLibrary.Conv_IntToDouble` (`self.Cnt_Spawn_Max`))))
  (set `self.Index_GenerateSection` (`KismetMathLibrary.RandomIntegerInRange` 1 (`self.Cnt_Spawn_Max`)))
  (bind _output_get (set `self.R_spawn` (`KismetMathLibrary.RandomFloatInRange` (`self.R_spawn_min`) (`self.R_spawn_max`)) :!label _label_2))
  (bind _returnvalue (`GameplayStatics.GetActorOfClass` "/Game/Blueprints/NewCar.NewCar_C"))
  (bind _yaw (.yaw (.rotation (`self.GetTransform` _returnvalue))))
  (bind _returnvalue_2 (- (`KismetMathLibrary.RandomFloatInRange` (* (`KismetMathLibrary.Conv_IntToDouble` (- (`self.Index_GenerateSection`) 1)) (`self.AngleRange`)) (* (`KismetMathLibrary.Conv_IntToDouble` (`self.Index_GenerateSection`)) (`self.AngleRange`))) _yaw))
  (bind _returnvalue_3 (`|SpawnActorFromClass` (`self.Item_AskedByTwitch`) (`KismetMathLibrary.MakeTransform` (`KismetMathLibrary.MakeVector` (.x (+ (.location (`self.GetTransform` _returnvalue)) (`KismetMathLibrary.MakeVector` (* _output_get (`KismetMathLibrary.DegSin` _returnvalue_2)) (* _output_get (`KismetMathLibrary.DegCos` _returnvalue_2))))) (.y (+ (.location (`self.GetTransform` _returnvalue)) (`KismetMathLibrary.MakeVector` (* _output_get (`KismetMathLibrary.DegSin` _returnvalue_2)) (* _output_get (`KismetMathLibrary.DegCos` _returnvalue_2)))))) (`KismetMathLibrary.MakeRotator` 0.0 0.0 (+ (`KismetMathLibrary.RandomFloatInRange` 85.0 95.0) _yaw))) "AdjustIfPossibleButDontSpawnIfColliding" "OverrideRootScale" null null))
  (`/Engine/EditorBlueprintResources/StandardMacros.IncrementInt` (`self.Cnt_Spawn`)
    (:`  `
      (`/Engine/EditorBlueprintResources/StandardMacros.IsValid` _returnvalue_3
        (:`Is Not Valid`
          (if (> (`self.Cnt_Spawn_Max`) (`self.Cnt_Spawn`))
            (bind _result (`/Engine/EditorBlueprintResources/StandardMacros.IncrementInt` (`self.Index_GenerateSection`))
              (:`  `
                (set `self.Index_GenerateSection` (mod _result (`self.Cnt_Spawn`)))
                (goto _label_2)))))))))

(event `SpawnRamp`
  ;[1 1 1] Generate Item by Twitch
  (bind _returnvalue (`GameplayStatics.GetActorOfClass` "/Game/Blueprints/NewCar.NewCar_C"))
  (bind _returnvalue_2 (`|SpawnActorFromClass` (`self.Item_AskedByTwitch`) (`KismetMathLibrary.MakeTransform` (`KismetMathLibrary.MakeVector` (.x (.location (`SceneComponent.K2_GetComponentToWorld` (`/Game/Blueprints/NewCar.SpawnPoint` _returnvalue)))) (.y (.location (`SceneComponent.K2_GetComponentToWorld` (`/Game/Blueprints/NewCar.SpawnPoint` _returnvalue))))) (`KismetMathLibrary.MakeRotator` 0.0 0.0 (.yaw (`self.K2_GetActorRotation` _returnvalue)))) "AlwaysSpawn" "OverrideRootScale" null null)))

(event `SpawnFuel`
  ;[1 1 1] Generate Item by Twitch
  (bind _returnvalue (`GameplayStatics.GetActorOfClass` "/Game/Blueprints/NewCar.NewCar_C"))
  (bind _returnvalue_2 (`|SpawnActorFromClass` (`self.Item_AskedByTwitch`) (`KismetMathLibrary.MakeTransform` (`KismetMathLibrary.MakeVector` (.x (.location (`SceneComponent.K2_GetComponentToWorld` (`/Game/Blueprints/NewCar.SpawnPoint` _returnvalue)))) (.y (.location (`SceneComponent.K2_GetComponentToWorld` (`/Game/Blueprints/NewCar.SpawnPoint` _returnvalue))))) (`KismetMathLibrary.MakeRotator` 0.0 0.0 (.yaw (`self.K2_GetActorRotation` _returnvalue)))) "AlwaysSpawn" "OverrideRootScale" null null)))

(event `SpawnMissile`
  (bind _returnvalue (`KismetMathLibrary.RandomFloatInRange` -10.0 10.0))
  ;[1 1 1] Generate Item by Twitch
  (set `self.Cnt_Spawn` 0)
  (set `self.AngleRange` (/ 180.0 (`KismetMathLibrary.Conv_IntToDouble` (`self.Cnt_Spawn_Max`))))
  (set `self.Index_GenerateSection` (`KismetMathLibrary.RandomIntegerInRange` 8 (- (`self.Cnt_Spawn_Max`) 8)))
  (bind _returnvalue_2 (`GameplayStatics.GetActorOfClass` "/Game/Blueprints/NewCar.NewCar_C"))
  (bind _returnvalue_3 (`ArcadeVehicleMovementComponentBase.GetCurrentSpeedAbsolute` (`StaticArcadeVehiclePawn.MovementComponent` _returnvalue_2)))
  (bind _output_get (set `self.R_spawn` (`KismetMathLibrary.SelectFloat` 200.0 (* (`KismetMathLibrary.RandomFloatInRange` (`self.R_spawn_min`) (`self.R_spawn_max`)) _returnvalue_3 0.03) (<= _returnvalue_3 10.0)) :!label _label_3))
  (bind _returnvalue_4 (- (`KismetMathLibrary.RandomFloatInRange` (* (`KismetMathLibrary.Conv_IntToDouble` (- (`self.Index_GenerateSection`) 1)) (`self.AngleRange`)) (* (`KismetMathLibrary.Conv_IntToDouble` (`self.Index_GenerateSection`)) (`self.AngleRange`))) (.yaw (.rotation (`self.GetTransform` _returnvalue_2)))))
  (bind _returnvalue_5 (`|SpawnActorFromClass` (`self.Item_AskedByTwitch`) (`KismetMathLibrary.MakeTransform` (`KismetMathLibrary.MakeVector` (.x (+ (.location (`self.GetTransform` _returnvalue_2)) (`KismetMathLibrary.MakeVector` (* _output_get (`KismetMathLibrary.DegSin` _returnvalue_4)) (* _output_get (`KismetMathLibrary.DegCos` _returnvalue_4))))) (.y (+ (.location (`self.GetTransform` _returnvalue_2)) (`KismetMathLibrary.MakeVector` (* _output_get (`KismetMathLibrary.DegSin` _returnvalue_4)) (* _output_get (`KismetMathLibrary.DegCos` _returnvalue_4))))) 500.0) (`KismetMathLibrary.MakeRotator` _returnvalue _returnvalue)) "AdjustIfPossibleButDontSpawnIfColliding" "OverrideRootScale" null null))
  (`/Engine/EditorBlueprintResources/StandardMacros.IncrementInt` (`self.Cnt_Spawn`)
    (:`  `
      (`/Engine/EditorBlueprintResources/StandardMacros.IsValid` _returnvalue_5
        (:`Is Not Valid`
          (if (> (`self.Cnt_Spawn_Max`) (`self.Cnt_Spawn`))
            (bind _result (`/Engine/EditorBlueprintResources/StandardMacros.IncrementInt` (`self.Index_GenerateSection`))
              (:`  `
                (set `self.Index_GenerateSection` (mod _result (`self.Cnt_Spawn`)))
                (goto _label_3)))))))))

(fn `UserConstructionScript`)