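; End position trigger actor that sends a NewCar back to the player start when it overlaps while the game has not started.
; Tick finds a NewCar in the world every frame and copies its IsGameStart flag.
; On overlap with that flag false, the car moves to PlayerStart's X and Y without sweep, keeping its vehicle mesh's current Z.
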(event `self.ReceiveActorBeginOverlap`
  (params (OtherActor :type "Actor Object Reference"))
  (if (not (`self.IsGameStart`))
    (bind _asnew_car (cast `/Game/Blueprints/NewCar` OtherActor))
    (`self.K2_SetActorLocation` _asnew_car (`KismetMathLibrary.MakeVector` (.x (`self.K2_GetActorLocation` (`self.PlayerStart`))) (.y (`self.K2_GetActorLocation` (`self.PlayerStart`))) (.z (`SceneComponent.K2_GetComponentLocation` (`StaticArcadeVehiclePawn.VehicleMesh` _asnew_car)))) false false)))

(event `self.ReceiveTick`
  (params (DeltaSeconds :type "Float (single-precision)"))
  (bind _returnvalue (`GameplayStatics.GetActorOfClass` "/Game/Blueprints/NewCar.NewCar_C"))
  (set `self.IsGameStart` (`/Game/Blueprints/NewCar.IsGameStart` _returnvalue)))

(fn `UserConstructionScript`)